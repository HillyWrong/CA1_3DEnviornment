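; BP_ShootingStars is an ambient sky effect actor that keeps spawning shooting star particle systems high around its location.
; From BeginPlay it runs an endless StarLife and SpawnStars event loop, waiting a short random delay between spawns.
; Each spawn places the ShootingStars system at a random wide horizontal and high vertical offset from the actor, with a slight fixed downward pitch.
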(event Custom|StarLife
  (Utilities|FlowControl|Delay (Math|Random|RandomFloatinRange 0.5 1.5))
  (CallFunction|SpawnStars))

(event Custom|SpawnStars
  (Niagara|SpawnSystematLocation "/Game/ShootingStars.ShootingStars" (+ (Transformation|GetActorLocation) (Math|Vector|MakeVector (Math|Random|RandomFloatinRange -2e+04 2e+04) (Math|Random|RandomFloatinRange -2e+04 2e+04) (Math|Random|RandomFloatinRange 8e+03 1.2e+04))) (Math|Rotator|MakeRotator 0.0 -15.0 0.0))
  (CallFunction|StarLife))

(event EventBeginPlay
  (CallFunction|StarLife))

(event Collision|EventActorBeginOverlap
  (params (OtherActor :type Actor%20Object%20Reference)))

(event EventTick
  (params (DeltaSeconds :type Float%20%28single-precision%29)))

(fn ConstructionScript)