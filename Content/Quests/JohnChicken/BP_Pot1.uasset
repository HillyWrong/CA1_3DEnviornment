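; BP_Pot1 is an interactable pot in the JohnChicken quest that responds once the player holds a key.
; A PickUpKey event sets HasKey, and Interact then toggles the mushroom's visibility a single time and plays the FixTent sound.
; The same interaction updates the first-person character's to-do list with a new mission and flags the TalkingDeer actor's TentFixed state.
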(event EventInteract
  (if (Variables|Default|GetHasKey?)
    (Utilities|FlowControl|DoOnce false
      (:Completed
        (Rendering|ToggleVisibility (Variables|Default|GetMushroom) false)
        (Audio|PlaySound2D "/Game/Sounds/FixTent.FixTent" 1.0 1.0 0.0 0 0)
        (bind _asbp_first_person_character (Utilities|Casting|CastToBP_FirstPersonCharacter (Game|GetPlayerCharacter 0)))
        (Utilities|FlowControl|DoOnce false
          (:Completed
            (Default|UpdatetoDo _asbp_first_person_character (Variables|Default|GetNewMissionToSet))
            (bind _returnvalue (Actor|GetActorOfClass "/Game/Dialouge/TalkingDeer.TalkingDeer_C"))
            (Variables|/Game/Dialouge/TalkingDeer.TalkingDeer_C|SetTentFixed? _returnvalue true)))))))

(event EventPickUpKey
  (Variables|Default|SetHasKey? true))

(fn ConstructionScript)