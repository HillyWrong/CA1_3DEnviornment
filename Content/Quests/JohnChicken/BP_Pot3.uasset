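; BP_Pot3 is a pot interactable in the JohnChicken quest that the player uses once a key has been picked up.
; PickUpKey sets HasKey and increments the Mushrooms counter on the first BP_Pot1 found in the level, printing the new count.
; Interact, gated by HasKey and a DoOnce, hides the Mushroom component and plays the FixTent sound.
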(event EventInteract
  (if (Variables|Default|GetHasKey?)
    (Utilities|FlowControl|DoOnce false
      (:Completed
        (Rendering|ToggleVisibility (Variables|Default|GetMushroom) false)
        (Audio|PlaySound2D "/Game/Sounds/FixTent.FixTent" 1.0 1.0 0.0 0 0)))))

(event EventPickUpKey
  (bind _returnvalue (Actor|GetActorOfClass "/Game/Quests/JohnChicken/BP_Pot1.BP_Pot1_C"))
  (bind _output_get (Variables|/Game/Quests/JohnChicken/BP_Pot1.BP_Pot1_C|SetMushrooms _returnvalue (+ (Variables|/Game/Quests/JohnChicken/BP_Pot1.BP_Pot1_C|GetMushrooms _returnvalue) 1.0)))
  (Variables|Default|SetHasKey? true)
  (Development|PrintString (Utilities|String|ToString(Float) _output_get)))

(fn ConstructionScript)