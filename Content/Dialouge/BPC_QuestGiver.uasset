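; Quest giver component that opens and closes the dialogue UI and relays dialogue triggers.
; StartDialouge creates WB_Dialouge_Main with a first row name and a self reference, then sets UI-only input, guarded by a DoOnce against reopening.
; EndConversation removes the widget, hides the cursor, restores game-only input and resets the guard.
; Dialougetrigger broadcasts non-None trigger names through the OnDialougeEventTriggered dispatcher.
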(event Custom|StartDialouge
  (params (FirstRowName :type Name))
  ;[0.15 0.15 0.15 0.5] Open Widget and change input mode to UI only
  (Utilities|FlowControl|DoOnce false
    (:Completed
      (bind _returnvalue (UserInterface|CreateWidget "/Game/Dialouge/WB_Dialouge_Main.WB_Dialouge_Main_C" 0 FirstRowName self))
      (bind _output_get (Variables|Default|SetDialouge_Widget _returnvalue))
      (UserInterface|Viewport|AddtoViewport _output_get 0)
      (Input|SetInputModeUIOnly (Game|GetPlayerController 0) _output_get "DoNotLock" false))))

(event Custom|EndConversation
  (bind _returnvalue (Game|GetPlayerController 0))
  ;[0.15 0.15 0.15 0.5] close widget and return to game mode
  (Widget|RemovefromParent (Variables|Default|GetDialouge_Widget))
  (Variables|/Script/Engine.PlayerController|SetbShowMouseCursor _returnvalue false)
  (Input|SetInputModeGameOnly _returnvalue false)
  (Variables|Default|SetDialouge_Widget 0)
  ;[0.15 0.15 0.15 0.5] Open Widget and change input mode to UI only
  (Utilities|FlowControl|DoOnce false) ; enters at Reset
)

(event Custom|Dialougetrigger
  (params (TriggerName :type Name))
  ;[0.15 0.15 0.15 0.5] Dialouge Event trigegr
  (if (!= TriggerName "")
    (Default|CallOnDialougeEventTriggered TriggerName)))

(fn ConstructionScript)