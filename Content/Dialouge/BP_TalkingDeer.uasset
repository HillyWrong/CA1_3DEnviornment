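; BP_TalkingDeer is an NPC deer that shows its dialogue lines in a UI widget, one per Speak call.
; Each call advances TalkIndex, creates the WB_Dialouge_Main widget if none is valid, sets its text and plays a 2D deer sound.
; Past the last line the widget is removed from its parent; the index is never reset here.
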(event EventSpeak
  ;[0.15 0.15 0.15 0.5] Displaying NPC Dialouge in UI Widget
  (Math|Integer|IncrementInt (Variables|Default|GetTalkIndex)
    (:%20%20
      (if (< (Variables|Default|GetTalkIndex) (Utilities|Array|Length (Variables|Default|GetDialouge)))
        (Variables|Default|GetUI
          (:then
            _)
          (:else
            (bind _returnvalue (UserInterface|CreateWidget "/Game/Dialouge/WB_Dialouge_Main.WB_Dialouge_Main_C" (Game|GetPlayerController 0)))
            (bind _output_get (Variables|Default|SetUI _returnvalue))
            (UserInterface|Viewport|AddtoViewport _output_get 0)))
        (Rendering|Components|TextRender|SetText (Variables|/Game/Dialouge/WB_Dialouge_Main.WB_Dialouge_Main_C|GetTalktext (Variables|Default|GetUI)) (Utilities|Text|ToText(String) (Utilities|Array|Get(acopy) (Variables|Default|GetDialouge) (Variables|Default|GetTalkIndex))))
        (Audio|PlaySound2D "/Game/Sounds/DeerSound.DeerSound" 1.0 1.0 0.0 0 0)
        (else
          (Widget|RemovefromParent (Variables|Default|GetUI)))))))

(fn ConstructionScript)